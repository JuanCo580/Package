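; Player actor with a physics cube that is pulled toward a planet and loads DeadLevel when LifeCount runs out.
; BeginPlay caches the first Planet_BP as Moon, and Tick adds a Gravity-scaled velocity toward it, without delta-time scaling.
; The Up input sets the UpPressed flag and toggles a particle system, but applies no thrust in this graph.
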(event `self.ReceiveBeginPlay`
  (bind _outactors (`GameplayStatics.GetAllActorsOfClass` "/Game/Objects/Planet_BP.Planet_BP_C"))
  (set `self.Moon` (`|GetArrayItem` _outactors)))

(event `self.ReceiveTick`
  (params (DeltaSeconds :type "Float (single-precision)"))
  (`|ExecutionSequence`
    (:`then_0`
      (if (<= (`self.lifeCount`) 0.0)
        (`GameplayStatics.OpenLevel` "DeadLevel")))
    (:`then_1`
      (`PrimitiveComponent.SetPhysicsLinearVelocity` (`self.Cube`) (* (* (`KismetMathLibrary.GetForwardVector` (`KismetMathLibrary.FindLookAtRotation` (`self.K2_GetActorLocation` (`self.Moon`)) (`self.K2_GetActorLocation`))) -1) (`self.Gravity`)) true (`self.Bone Name`)))))

(event `InputAction|Up`
  (params (Key :type "Key Structure"))
  (bind _particlesystem (`self.ParticleSystem`))
  (:`Pressed`
    (set `self.upPressed` true)
    (`ActorComponent.Activate` _particlesystem true))
  (:`Released`
    (set `self.upPressed` false)
    (`ActorComponent.Deactivate` _particlesystem)))

(fn `UserConstructionScript`)